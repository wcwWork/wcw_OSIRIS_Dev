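; Test actor that exercises Osiris subsystem snapshot save and load on itself and its components.
; On BeginPlay it randomizes Health, TempCounter and the inventory component's Gold, saves a snapshot, re-randomizes them after a delay, then loads the snapshot.
; Printed values at each stage show whether Health and component Gold are restored, with TempCounter labeled as the unsaved control.
; Failed saves or loads print an error message.
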(event `self.ReceiveBeginPlay`
  (set `self.Health` (`KismetMathLibrary.RandomFloatInRange` 1.0 100.0))
  (set `self.TempCounter` (`KismetMathLibrary.RandomIntegerInRange` 1 100))
  (set `/Game/BPC_TestInventory.Gold` (`KismetMathLibrary.RandomIntegerInRange` 1 100) (`self.BPC_TestInventory`))
  (`KismetSystemLibrary.PrintString` (`KismetStringLibrary.Concat_StrStr` " Health(SAVE): " (`KismetStringLibrary.Conv_DoubleToString` (`self.Health`))) true false (struct :`R` 0.230327 :`G` 1.0 :`A` 1.0) 5.0)
  (`KismetSystemLibrary.PrintString` (`KismetStringLibrary.Concat_StrStr` " TempCounter(NO SAVE): " (`KismetStringLibrary.Conv_IntToString` (`self.TempCounter`))) true false (struct :`R` 0.230327 :`G` 1.0 :`A` 1.0) 5.0)
  (`KismetSystemLibrary.PrintString` (`KismetStringLibrary.Concat_StrStr` " Gold from BPC(SAVE): " (`KismetStringLibrary.Conv_IntToString` (`/Game/BPC_TestInventory.Gold` (`self.BPC_TestInventory`)))) true false (struct :`R` 0.230327 :`G` 1.0 :`A` 1.0) 5.0)
  (bind _returnvalue (`OsirisSubsystem.SaveGameSnapshot` (subsystem `OsirisSubsystem`) self true))
  (if _returnvalue
    (`KismetSystemLibrary.Delay` 5.0)
    (set `self.Health` (`KismetMathLibrary.RandomFloatInRange` 1.0 100.0))
    (set `self.TempCounter` (`KismetMathLibrary.RandomIntegerInRange` 1 100))
    (set `/Game/BPC_TestInventory.Gold` (`KismetMathLibrary.RandomIntegerInRange` 1 100) (`self.BPC_TestInventory`))
    (`KismetSystemLibrary.PrintString` (`KismetStringLibrary.Concat_StrStr` " Health(MUTATED IN RUNTIME): " (`KismetStringLibrary.Conv_DoubleToString` (`self.Health`))) true false (struct :`R` 1.0 :`G` 0.11841 :`A` 1.0) 10.0)
    (`KismetSystemLibrary.PrintString` (`KismetStringLibrary.Concat_StrStr` " TempCounter(MUTATED IN RUNTIME): " (`KismetStringLibrary.Conv_IntToString` (`self.TempCounter`))) true false (struct :`R` 1.0 :`G` 0.11841 :`A` 1.0) 10.0)
    (`KismetSystemLibrary.PrintString` (`KismetStringLibrary.Concat_StrStr` " Gold from BPC(MUTATED IN RUNTIME): " (`KismetStringLibrary.Conv_IntToString` (`/Game/BPC_TestInventory.Gold` (`self.BPC_TestInventory`)))) true false (struct :`R` 1.0 :`G` 0.11841 :`A` 1.0) 10.0)
    (`KismetSystemLibrary.Delay` 10.0)
    (if (`OsirisSubsystem.LoadGameSnapshot` (subsystem `OsirisSubsystem`) self true)
      (`KismetSystemLibrary.PrintString` "Apply Load Game Snapshot!" true false (struct :`R` 0.079981 :`G` 1.0 :`A` 1.0))
      (`KismetSystemLibrary.Delay` 0.1)
      (`KismetSystemLibrary.PrintString` (`KismetStringLibrary.Concat_StrStr` " Health(LOAD): " (`KismetStringLibrary.Conv_DoubleToString` (`self.Health`))) true false (struct :`R` 0.022959 :`G` 1.0 :`A` 1.0) 10.0)
      (`KismetSystemLibrary.PrintString` (`KismetStringLibrary.Concat_StrStr` " TempCounter(NO SAVE): " (`KismetStringLibrary.Conv_IntToString` (`self.TempCounter`))) true false (struct :`R` 0.022959 :`G` 1.0 :`A` 1.0) 10.0)
      (`KismetSystemLibrary.PrintString` (`KismetStringLibrary.Concat_StrStr` " Gold from BPC(LOAD): " (`KismetStringLibrary.Conv_IntToString` (`/Game/BPC_TestInventory.Gold` (`self.BPC_TestInventory`)))) true false (struct :`R` 0.022959 :`G` 1.0 :`A` 1.0) 10.0)
      (else
        (`KismetSystemLibrary.PrintString` "Load Game Snapshot is Failed!" true false (struct :`R` 1.0 :`G` 0.025299 :`A` 1.0))))
    (else
      (`KismetSystemLibrary.PrintString` " Save Game Snapshot is Failed!" true false (struct :`R` 1.0 :`G` 0.025299 :`A` 1.0)))))

(fn `UserConstructionScript`)