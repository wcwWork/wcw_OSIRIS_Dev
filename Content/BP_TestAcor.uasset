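; BP_TestAcor is a test actor that randomizes its own state at BeginPlay, with a looping timer firing a MUTATED event to repeat it.
; Each mutation rerolls a test number, teleports to a random navigable point nearby with random rotation, swaps its mesh between cone and cube, and randomizes the inventory component's Gold.
; Tick prints the test number and Gold to screen every frame.
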(event `self.ReceiveBeginPlay`
  (bind _returnvalue_location (`KismetMathLibrary.BreakTransform` (`self.GetTransform`)))
  (`KismetSystemLibrary.K2_SetTimerDelegate` (delegate `MUTATED`) 5.0 true)
  (set `self.TestNumber` (`KismetMathLibrary.RandomIntegerInRange` 1 99) :!label _label)
  (bind _randomlocation (`NavigationSystemV1.K2_GetRandomLocationInNavigableRadius` _returnvalue_location 500.0 null null))
  (`self.K2_SetActorTransform` (`KismetMathLibrary.MakeTransform` _randomlocation (`KismetMathLibrary.MakeRotator` (`KismetMathLibrary.RandomFloatInRange` -180.0 180.0) (`KismetMathLibrary.RandomFloatInRange` -180.0 180.0) (`KismetMathLibrary.RandomFloatInRange` -180.0 180.0))) false true)
  (bind _staticmesh (`self.StaticMesh`)
    (:`then`
      (`StaticMeshComponent.SetStaticMesh` _staticmesh (select `int` (`KismetMathLibrary.RandomIntegerInRange` 0 1) :`0` "/Engine/BasicShapes/Cone.Cone" :`1` "/Engine/BasicShapes/Cube.Cube" :!type "StaticMesh Object Reference")))
    (:`else`
      _))
  (bind _bpc_testinventory (`self.BPC_TestInventory`)
    (:`then`
      (set `/Game/BPC_TestInventory.Gold` (`KismetMathLibrary.RandomIntegerInRange` 1 99) _bpc_testinventory))
    (:`else`)))

(event `MUTATED`
  (goto _label))

(event `self.ReceiveTick`
  (params (DeltaSeconds :type "Float (single-precision)"))
  (`|ExecutionSequence`
    (:`then_0`
      (`KismetSystemLibrary.PrintString` (`KismetStringLibrary.Concat_StrStr` "TestNum: " (`KismetStringLibrary.Conv_IntToString` (`self.TestNumber`))) true false (struct :`R` 0.061246 :`G` 0.250158 :`B` 0.184475 :`A` 1.0) 0.0))
    (:`then_1`
      (bind _bpc_testinventory (`self.BPC_TestInventory`)
        (:`then`
          (`KismetSystemLibrary.PrintString` (`KismetStringLibrary.Concat_StrStr` "Gold: " (`KismetStringLibrary.Conv_IntToString` (`/Game/BPC_TestInventory.Gold` _bpc_testinventory))) true false (struct :`R` 1.0 :`G` 0.46388 :`A` 1.0) 0.0))
        (:`else`)))))

(fn `UserConstructionScript`)